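; Projectile actor that destroys enemies on contact and awards points to the player.
; A capsule overlap with an Enemy destroys both actors, then adds to the Score and TempScore of BP_Player, the first player's pawn.
; A lifespan set at BeginPlay removes stray projectiles, while Tick increments and clamps the movement component's InitialSpeed.
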(event OnComponentBeginOverlap(Capsule)
  (params (OverlappedComponent :type Primitive%20Component%20Object%20Reference) (OtherActor :type Actor%20Object%20Reference) (OtherComp :type Primitive%20Component%20Object%20Reference) (OtherBodyIndex :type Integer) (bFromSweep :type Boolean) (SweepResult :type Hit%20Result%20Structure%20%28by%20ref%29))
  (bind _asenemy (Utilities|Casting|CastToEnemy OtherActor))
  (Actor|DestroyActor _asenemy)
  (Actor|DestroyActor)
  (bind _asbp_player (Utilities|Casting|CastToBP_Player (Game|Player|GetPlayerPawn 0)))
  (Variables|/Game/InfiniteMatrix/Blueprints/BP_Player.BP_Player_C|SetScore _asbp_player (+ (Variables|/Game/InfiniteMatrix/Blueprints/BP_Player.BP_Player_C|GetScore _asbp_player) 2))
  (Variables|/Game/InfiniteMatrix/Blueprints/BP_Player.BP_Player_C|SettempScore _asbp_player (+ (Variables|/Game/InfiniteMatrix/Blueprints/BP_Player.BP_Player_C|GettempScore _asbp_player) 2)))

(event EventBeginPlay
  (Actor|SetLifeSpan 2e+02))

(event Collision|EventActorBeginOverlap
  (params (OtherActor :type Actor%20Object%20Reference)))

(event EventTick
  (params (DeltaSeconds :type Float%20%28single-precision%29))
  (bind _projectilemovement (Variables|Default|GetProjectileMovement))
  (Variables|/Script/Engine.ProjectileMovementComponent|SetInitialSpeed _projectilemovement (Math|Float|Clamp(Float) (+ (Variables|/Script/Engine.ProjectileMovementComponent|GetInitialSpeed _projectilemovement) 1.0))))

(fn ConstructionScript)